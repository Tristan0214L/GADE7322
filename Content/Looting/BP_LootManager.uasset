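; BP_LootManager picks random item drops from ItemTable and records each in DroppedItems.
; GenerateLoot applies one reroll mode by priority: NoDupes retries duplicates many times, RerollDupes only briefly, and EmptySlots targets item types already dropped.
; All retries are capped, so repeats remain possible.
; SameSlot is never cleared inside GenerateLoot, so an EmptySlots match rerolls to the cap regardless of new picks.
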(fn `GenerateLoot`
  (params (NoDupes :type Boolean) (RerollDupes :type Boolean) (EmptySlots :type Boolean))
  (returns (Item :type "/Game/Looting/FItemData Structure"))
  (locals (tempCounter :type Integer) (tempDrop :type "/Game/Looting/FItemData Structure") (sameSlot :type Boolean))
  (bind _droppeditems (`self.DroppedItems`))
  (bind _tempdrop (`local.tempDrop`))
  (set `local.tempCounter` 0)
  (bind _output_get (set `local.tempDrop` (`KismetArrayLibrary.Array_Random` (`self.ItemTable`))))
  (if NoDupes
    (bind _returnvalue (`KismetArrayLibrary.Array_Contains` _droppeditems _output_get))
    (while (and (< (`local.tempCounter`) 20) _returnvalue)
      (set `local.tempDrop` (`KismetArrayLibrary.Array_Random` (`self.ItemTable`)) :!label _label)
      (`/Engine/EditorBlueprintResources/StandardMacros.IncrementInt` (`local.tempCounter`)))
    (elif RerollDupes
      (while (and _returnvalue (< (`local.tempCounter`) 2))
        (goto _label))
      (elif EmptySlots
        (for _array_element (`self.DroppedItems`)
          (if (`|EnumEquality` (`.EItemType_12_018F6BD54003C65E44352085C9BEB126` (break `/Game/Looting/FItemData` (`local.tempDrop`))) (`.EItemType_12_018F6BD54003C65E44352085C9BEB126` (break `/Game/Looting/FItemData` _array_element)))
            (set `local.sameSlot` true)))
        (while (and (`local.sameSlot`) (< (`local.tempCounter`) 5))
          (for _array_element_2 (`self.DroppedItems`)
            (if (`|EnumEquality` (`.EItemType_12_018F6BD54003C65E44352085C9BEB126` (break `/Game/Looting/FItemData` (`local.tempDrop`))) (`.EItemType_12_018F6BD54003C65E44352085C9BEB126` (break `/Game/Looting/FItemData` _array_element_2)))
              (set `local.sameSlot` true)))
          (goto _label)))))
  (`KismetArrayLibrary.Array_Add` _droppeditems _tempdrop)
  (return _tempdrop))

(fn `UserConstructionScript`)